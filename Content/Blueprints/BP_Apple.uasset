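; BP_Apple is an apple actor that reacts to being hit by a Demo_Test actor, using Kinect hand tracking.
; On hit it prints a debug message and checks the centered body's left hand state.
; Only the Unknown state acts, setting the apple's relative location to its scale vector.
; Physics handle and destroy nodes are unconnected, so the graph looks like an unfinished prototype.
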(event `self.M_Apple.OnComponentHit`
  (params (HitComponent :type "PrimitiveComponent Object Reference") (OtherActor :type "Actor Object Reference") (OtherComp :type "PrimitiveComponent Object Reference") (NormalImpulse :type "Vector Structure") (Hit :type "HitResult Structure (by ref)"))
  (cast `/Game/Blueprints/BP_Demo_Test` OtherActor)
  (`KismetSystemLibrary.PrintString` "Hello")
  (bind _centeredbody (`KinectInterfaceComponent.GetCenteredBody` (`self.KinectInterface`)))
  (`KinectInterfaceComponent.GetHandStateAsExecution` (`self.KinectInterface`) "Left" _centeredbody
    (:`Unknown`
      (`self.K2_SetActorRelativeLocation` (`ActorComponent.GetOwner` (`self.M_Apple`)) (`self.GetActorRelativeScale3D`) false false))))

(fn `UserConstructionScript`)