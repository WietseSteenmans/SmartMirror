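; BP_Demo_Test is a test Blueprint that moves two hand meshes to follow a player's hands tracked by Kinect.
; Every Tick it asks the KinectInterface for the centered body, then reads that body's absolute left and right hand joint positions.
; Those positions are applied directly as relative locations of LeftHandMesh and RightHandMesh, with no sweep, smoothing or check that a body is tracked.
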(event `self.ReceiveTick`
  (params (DeltaSeconds :type "Float (single-precision)"))
  (bind _centeredbody (`KinectInterfaceComponent.GetCenteredBody` (`self.KinectInterface`)))
  (bind _returnvalue (`KinectInterfaceComponent.GetJointAbsolutePosition` (`self.KinectInterface`) "HandLeft" _centeredbody))
  (`SceneComponent.K2_SetRelativeLocation` (`self.LeftHandMesh`) _returnvalue false false)
  (bind _returnvalue_2 (`KinectInterfaceComponent.GetJointAbsolutePosition` (`self.KinectInterface`) "HandRight" _centeredbody))
  (`SceneComponent.K2_SetRelativeLocation` (`self.RightHandMesh`) _returnvalue_2 false false))

(fn `UserConstructionScript`)